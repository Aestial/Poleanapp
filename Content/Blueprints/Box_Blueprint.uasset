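; Clickable board box actor that holds stacked chips and shows a configurable text label set in the construction script.
; Cursor hover toggles a crosshair cursor plus mesh and particle highlights, and a click calls BoxClicked with the box location and plays a chip sound.
; Overlaps maintain a chip count that gives each arriving chip its stack floor, though increments count any actor while decrements count only chips.
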(event `self.ReceiveActorBeginCursorOver`
  ;[1 1 1] MouseOver. Changes cursor and material.
  (set `PlayerController.CurrentMouseCursor` "Crosshairs" (`GameplayStatics.GetPlayerController` 0))
  (`SceneComponent.SetVisibility` (`self.HoverMark`) true false)
  (`SceneComponent.SetVisibility` (`self.ParticleMark`) true false))

(event `self.ReceiveActorEndCursorOver`
  ;[1 1 1] MouseOver. Changes cursor and material.
  (set `PlayerController.CurrentMouseCursor` "Default" (`GameplayStatics.GetPlayerController` 0))
  (`SceneComponent.SetVisibility` (`self.HoverMark`) false false)
  (`SceneComponent.SetVisibility` (`self.ParticleMark`) false false))

(event `self.ReceiveActorOnClicked`
  (params (ButtonPressed :type "Key Structure" :default "AnyKey"))
  ;[1 1 1] Clicked
  (`self.BoxClicked` (`self.K2_GetActorLocation`))
  (`GameplayStatics.SpawnSoundAttached` "/Game/Assets/Sounds/ChipPush_Stereo_Cue.ChipPush_Stereo_Cue" (`self.TriggerVolume`)))

(event `self.ReceiveActorBeginOverlap`
  (params (OtherActor :type "Actor Object Reference"))
  (bind _chips (`self.Chips`))
  (set `self.Chips` (+ _chips 1))
  (if (< 0 _chips)
    (bind _aschip_blueprint (cast `/Game/Blueprints/Chip_Blueprint` OtherActor))
    (`/Game/Blueprints/Chip_Blueprint.SetFloor` _aschip_blueprint (- _chips 1))))

(event `self.ReceiveActorEndOverlap`
  (params (OtherActor :type "Actor Object Reference"))
  (cast `/Game/Blueprints/Chip_Blueprint` OtherActor)
  (set `self.Chips` (- (`self.Chips`) 1)))

(fn `UserConstructionScript`
  (bind _label (`self.Label`))
  (`TextRenderComponent.K2_SetText` _label (`KismetTextLibrary.Conv_StringToText` (`self.LabelValue`)))
  (`TextRenderComponent.SetTextMaterial` _label (`self.LabelMaterial`))
  (`TextRenderComponent.SetTextRenderColor` _label (`KismetMathLibrary.Conv_LinearColorToColor` (`self.LabelColor`))))