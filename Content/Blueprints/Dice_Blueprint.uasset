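; Physics dice actor that rolls, reads its top face and shows the value as color-matched floating text.
; While Roll is set, Tick spins it randomly, then after delays enables gravity, applies forward force and marks it thrown.
; At zero velocity, it fires effects and Stopped, then matches actor axes against world Z to find the face.
; A runtime text component billboards toward the camera until Pick removes it and restores the starting transform.
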(event `self.ReceiveBeginPlay`
  ;[1 1 1] Pick dice. Set original position and event for picking
  (set `self.OriginalLocation` (`self.K2_GetActorLocation`))
  (set `self.OriginalRotation` (`self.K2_GetActorRotation`)))

(event `Pick`
  ;[1 1 1] Pick dice. Set original position and event for picking
  (set `self.ValueShown` false)
  (`ActorComponent.K2_DestroyComponent` (`self.TopValue_TR`))
  (`self.K2_SetActorLocationAndRotation` (`self.OriginalLocation`) (`self.OriginalRotation`)))

(event `self.ReceiveTick`
  (params (DeltaSeconds :type "Float (single-precision)"))
  (bind _staticmesh (`self.StaticMesh`))
  (bind _topvalue_tr (`self.TopValue_TR`))
  (bind _transformcomponent (`PlayerCameraManager.TransformComponent` (`GameplayStatics.GetPlayerCameraManager` 0)))
  (bind _relativelocation (`SceneComponent.RelativeLocation` _transformcomponent))
  (`|ExecutionSequence`
    (:`then_0`
      ;[1 1 1] Rolls dice. Add random rotation, enable gravity and add linear force.
      (if (`self.Roll`)
        (`self.K2_AddActorLocalRotation` (`KismetMathLibrary.RandomRotator` false))
        (`|ExecutionSequence`
          (:`then_0`
            (`KismetSystemLibrary.Delay` (`self.RollingDuration`))
            (set `self.Roll` false)
            (set `self.Thrown` true))
          (:`then_1`
            (`KismetSystemLibrary.Delay` (`self.GravityDelay`))
            (`PrimitiveComponent.SetEnableGravity` _staticmesh true)
            (`PrimitiveComponent.AddForce` _staticmesh (`KismetMathLibrary.MakeVector` (`KismetMathLibrary.RandomFloatInRange` 14500.0 16500.0)) "None" false)))))
    (:`then_1`
      ;[1 1 1] Check when dice stops, activates effect, checks top value and send event to UI.
      (if (and (== (`self.GetVelocity`) (0.0 0.0 0.0) :`ErrorTolerance` 0.0) (`self.Thrown`))
        (`|ExecutionSequence`
          (:`then_0`
            (`ActorComponent.Activate` (`self.Effect`) false)
            (`self.Stopped`))
          (:`then_1`
            (`ActorComponent.Activate` (`self.EffectAudio`) false)
            (set `self.Thrown` false))
          (:`then_2`
            (`self.GetTopValue`)
            (`self.DisplayTopValue`)))))
    (:`then_2`
      ;[1 1 1] Value TR billboarding. Rotates towards camera.
      (if (`self.ValueShown`)
        (set `SceneComponent.bAbsoluteLocation` true _transformcomponent)
        (`|ExecutionSequence`
          (:`then_0`
            (if (`self.ShowDebug`)
              (`KismetSystemLibrary.DrawDebugString` (0.0 0.0 0.0) (`KismetStringLibrary.Conv_VectorToString` _relativelocation))))
          (:`then_1`
            (set `SceneComponent.bAbsoluteRotation` true _topvalue_tr)
            (`SceneComponent.K2_SetWorldRotation` _topvalue_tr (`KismetMathLibrary.MakeRotFromX` (* (- (`self.K2_GetActorLocation`) _relativelocation) -1.0)) false)))))))

(fn `DebugDirection`
  (bind _returnvalue (`self.K2_GetActorLocation`))
  (bind _color_0 (`self.Color_0`))
  (if (`self.ShowDebug`)
    (`KismetSystemLibrary.DrawDebugString` (+ _returnvalue (0.0 0.0 90.0)) (`KismetStringLibrary.Conv_VectorToString` (`self.GetActorUpVector`)) null _color_0 0.0)
    (`KismetSystemLibrary.DrawDebugString` (+ _returnvalue (0.0 0.0 50.0)) (`KismetStringLibrary.Conv_VectorToString` (`self.GetActorForwardVector`)) null _color_0 0.0)
    (`KismetSystemLibrary.DrawDebugString` (+ _returnvalue (0.0 0.0 10.0)) (`KismetStringLibrary.Conv_VectorToString` (`self.GetActorRightVector`)) null _color_0 0.0)))

(fn `DisplayTopValue`
  (`|ExecutionSequence`
    (:`then_0`
      ;[1 1 1] Debug Display
      (if (`self.ShowDebug`)
        (`KismetSystemLibrary.DrawDebugString` (+ (`self.K2_GetActorLocation`) (0.0 0.0 5.0)) (`KismetStringLibrary.Conv_IntToString` (`self.TopValue`)) null (`self.Color_0`) 10.0)))
    (:`then_1`
      ;[1 1 1] Text Render Display
      (bind _returnvalue (`AddComponent|TextRenderComponent_4` :`bManualAttachment` true))
      (`|ExecutionSequence`
        (:`then_0`
          (`TextRenderComponent.K2_SetText` _returnvalue (`KismetTextLibrary.Conv_IntToText` (`self.TopValue`)))
          (`PrimitiveComponent.SetMaterial` _returnvalue 0 "/Game/Materials/M_EmissiveText.M_EmissiveText")
          (`TextRenderComponent.SetTextRenderColor` _returnvalue (`KismetMathLibrary.Conv_LinearColorToColor` (`self.Color_0`))))
        (:`then_1`
          (`SceneComponent.K2_SetWorldLocation` _returnvalue (`self.K2_GetActorLocation`) false)
          (`TextRenderComponent.SetWorldSize` _returnvalue 128.0))
        (:`then_2`
          (`SceneComponent.K2_AddLocalOffset` _returnvalue (0.0 0.0 175.0) false)
          (`TextRenderComponent.SetHorizontalAlignment` _returnvalue "EHTA_Center"))
        (:`then_3`
          (`SceneComponent.K2_AttachTo` _returnvalue (`self.StaticMesh`) "None" "KeepWorldPosition" true)
          (set `self.ValueShown` true)
          (set `self.TopValue_TR` _returnvalue))))))

(fn `GetTopValue`
  (bind _tolerance (`self.Tolerance`))
  (bind _z (.z (`self.GetActorForwardVector`)))
  (bind _z_2 (.z (`self.GetActorUpVector`)))
  (bind _z_3 (.z (`self.GetActorRightVector`)))
  (if (`KismetMathLibrary.NearlyEqual_FloatFloat` _z_2 1.0 _tolerance)
    (set `self.TopValue` 1)
    (elif (`KismetMathLibrary.NearlyEqual_FloatFloat` _z_2 -1.0 _tolerance)
      (set `self.TopValue` 6)
      (elif (`KismetMathLibrary.NearlyEqual_FloatFloat` _z 1.0 _tolerance)
        (set `self.TopValue` 4)
        (elif (`KismetMathLibrary.NearlyEqual_FloatFloat` _z -1.0 _tolerance)
          (set `self.TopValue` 3)
          (elif (`KismetMathLibrary.NearlyEqual_FloatFloat` _z_3 1.0 _tolerance)
            (set `self.TopValue` 5)
            (elif (`KismetMathLibrary.NearlyEqual_FloatFloat` _z_3 -1.0 _tolerance)
              (set `self.TopValue` 2)
              (else
                (set `self.TopValue` 0)))))))))

(fn `UserConstructionScript`
  (bind _returnvalue (`PrimitiveComponent.CreateDynamicMaterialInstance` (`self.StaticMesh`) 0 "/Game/Materials/M_Dice_LED_Inst.M_Dice_LED_Inst"))
  (`MaterialInstanceDynamic.SetVectorParameterValue` _returnvalue "Color" (`self.Color_0`))
  (`TextRenderComponent.SetTextRenderColor` (`self.TopValue_TR`) (`KismetMathLibrary.Conv_LinearColorToColor` (`self.Color_0`))))