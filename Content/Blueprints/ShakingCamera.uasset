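; ShakingCamera is an actor that tilts its camera to follow the mouse cursor.
; A gate opens three seconds after BeginPlay, letting Tick map the normalized cursor position to relative pitch and yaw within configurable half-angles.
; Rotation updates only while the cursor is inside a limited screen region.
; Despite the name, nothing shakes: a time-based sine sway is left unconnected, though its timer still accumulates.
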(event `self.ReceiveBeginPlay`
  (bind _halfangley (`self.HalfAngleY`))
  (bind _halfanglex (`self.HalfAngleX`))
  (bind (_locationx _locationy) (`PlayerController.GetMousePosition` (`GameplayStatics.GetPlayerController` 0)))
  (bind (_x _y) (`KismetMathLibrary.BreakVector2D` (`WidgetLayoutLibrary.GetViewportSize`)))
  (bind _returnvalue (/ _locationy _y))
  (bind _returnvalue_2 (/ _locationx _x))
  (`KismetSystemLibrary.Delay` 3.0)
  (goto _label :!via `Open`))

(event `self.ReceiveTick`
  (params (DeltaSeconds :type "Float (single-precision)"))
  (bind _halfangley (`self.HalfAngleY`))
  (bind _halfanglex (`self.HalfAngleX`))
  (bind (_locationx _locationy) (`PlayerController.GetMousePosition` (`GameplayStatics.GetPlayerController` 0)))
  (bind (_x _y) (`KismetMathLibrary.BreakVector2D` (`WidgetLayoutLibrary.GetViewportSize`)))
  (bind _returnvalue (/ _locationy _y))
  (bind _returnvalue_2 (/ _locationx _x))
  (`/Engine/EditorBlueprintResources/StandardMacros.Gate` true :!label _label
    (:`Exit`
      (set `self.Time` (+ DeltaSeconds (`self.Time`)))
      (if (and (`KismetMathLibrary.InRange_FloatFloat` _returnvalue_2 0.5) (`KismetMathLibrary.InRange_FloatFloat` _returnvalue 0.2 0.6))
        (`SceneComponent.SetRelativeRotation` (`self.Camera`) (`KismetMathLibrary.MakeRot` (`KismetMathLibrary.MapRange` _returnvalue 0.0 1.0 (* _halfangley -1.0) _halfangley) (`KismetMathLibrary.MapRange` _returnvalue_2 0.0 1.0 (* _halfanglex -1.0) _halfanglex)) false)))))

(fn `UserConstructionScript`)