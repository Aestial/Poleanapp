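; Clickable game chip actor that toggles selection and gives hover and selection feedback through materials, mouse cursors and a select sound.
; The construction script sets the material from ColorOption, and BeginPlay caches it for restoring when an unselected chip loses hover.
; Clicks fire ChipSelected or ChipUnselected calls; Deselect clears selection with a supplied material.
; SetFloor offsets the mesh vertically in fixed steps per floor.
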(event `self.ReceiveBeginPlay`
  ;[1 1 1] Begin Play. Get the chip's original material and storage it.
  (set `self.OriginalMaterial` (`KismetArrayLibrary.Array_Get` (`MeshComponent.OverrideMaterials` (`self.StaticMesh`)))))

(event `self.ReceiveActorOnClicked`
  (params (ButtonPressed :type "Key Structure" :default "AnyKey"))
  (bind _returnvalue (`GameplayStatics.GetPlayerController` 0))
  (bind _staticmesh (`self.StaticMesh`))
  ;[1 1 1] Click: Select Chip
  (if (`self.Selected`)
    (`|ExecutionSequence`
      (:`then_0`
        (`self.Deselect` "/Game/Materials/M_Chip_Hover_Inst.M_Chip_Hover_Inst")
        (`self.ChipUnselected`))
      (:`then_1`
        (set `PlayerController.CurrentMouseCursor` "GrabHand" _returnvalue)))
    (else
      (`|ExecutionSequence`
        (:`then_0`
          (`self.ChipSelected`))
        (:`then_1`
          (set `self.Selected` true)
          (`PrimitiveComponent.SetMaterial` _staticmesh 0 "/Game/Materials/M_Chip_Selected_Inst.M_Chip_Selected_Inst")
          (`GameplayStatics.SpawnSoundAttached` "/Game/Assets/Sounds/Frontend_ChipSelect_Stereo_Cue.Frontend_ChipSelect_Stereo_Cue" _staticmesh))
        (:`then_2`
          (set `PlayerController.CurrentMouseCursor` "GrabHandClosed" _returnvalue))))))

(event `self.ReceiveActorBeginCursorOver`
  (bind _returnvalue (`GameplayStatics.GetPlayerController` 0))
  ;[1 1 1] MouseOver. Changes cursor and material.
  (if (`self.Selected`)
    (set `PlayerController.CurrentMouseCursor` "GrabHandClosed" _returnvalue)
    (else
      (set `PlayerController.CurrentMouseCursor` "GrabHand" _returnvalue)
      (`PrimitiveComponent.SetMaterial` (`self.StaticMesh`) 0 "/Game/Materials/M_Chip_Hover_Inst.M_Chip_Hover_Inst"))))

(event `self.ReceiveActorEndCursorOver`
  ;[1 1 1] MouseOver. Changes cursor and material.
  (if (not (`self.Selected`))
    (set `PlayerController.CurrentMouseCursor` "Default" (`GameplayStatics.GetPlayerController` 0))
    (`PrimitiveComponent.SetMaterial` (`self.StaticMesh`) 0 (`self.OriginalMaterial`))))

(fn `Deselect`
  (params (SelectionMaterial :type "MaterialInterface Object Reference"))
  (set `self.Selected` false)
  (`PrimitiveComponent.SetMaterial` (`self.StaticMesh`) 0 SelectionMaterial))

(fn `SetFloor`
  (params (Floor :type Integer))
  (`SceneComponent.K2_SetRelativeLocation` (`self.StaticMesh`) (`KismetMathLibrary.MakeVector` 0.0 0.0 (* Floor 25.0)) false false))

(fn `UserConstructionScript`
  (`PrimitiveComponent.SetMaterial` (`self.StaticMesh`) 0 (select `int` (`self.ColorOption`) :`0` "/Game/Materials/M_Chip_Blue_Inst.M_Chip_Blue_Inst" :`1` "/Game/Materials/M_Chip_Green_Inst.M_Chip_Green_Inst" :`2` "/Game/Materials/M_Chip_Red_Inst.M_Chip_Red_Inst" :`3` "/Game/Materials/M_Chip_Yellow_Inst.M_Chip_Yellow_Inst" :!type "MaterialInterface Object Reference")))