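; Player controller for Poleana that lets the player look around with the mouse while the right button is held.
; Pressing or releasing the right mouse button sets a MousePress flag and shows the cursor only when the button is up.
; The Turn and LookUp axis inputs feed yaw and pitch input only while that flag is set.
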(event `InputAxis|Turn`
  (params (AxisValue :type "Float (single-precision)"))
  (if (`self.MousePress`)
    (`self.AddYawInput` AxisValue)))

(event `InputAxis|LookUp`
  (params (AxisValue :type "Float (single-precision)"))
  (if (`self.MousePress`)
    (`self.AddPitchInput` AxisValue)))

(event `Key|RightMouseButton`
  (params (Key :type "Key Structure" :default "AnyKey"))
  (:`Pressed`
    (set `self.MousePress` true)
    (set `self.bShowMouseCursor` (not (`self.MousePress`)) :!label _label))
  (:`Released`
    (set `self.MousePress` false)
    (goto _label)))

(fn `UserConstructionScript`)