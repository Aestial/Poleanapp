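; SideCharacter is a character Blueprint whose graph handles mouse wheel camera zoom.
; Wheel down shortens the DistanceArm length and wheel up lengthens it, each checked against a fixed distance limit.
; Each press applies a single FInterpTo step using ZoomScale, ZoomSpeed and world delta time, so zoom is not smoothed across frames.
; The construction script is empty.
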(event `Key|MouseScrollDown`
  (params (Key :type "Key Structure" :default "AnyKey"))
  (bind _distancearm (`self.DistanceArm`))
  (bind _targetarmlength (`SpringArmComponent.TargetArmLength` _distancearm))
  (:`Pressed`
    (if (> _targetarmlength 450.0)
      (set `SpringArmComponent.TargetArmLength` (`KismetMathLibrary.FInterpTo` _targetarmlength (- _targetarmlength (`self.ZoomScale`)) (`GameplayStatics.GetWorldDeltaSeconds`) (`self.ZoomSpeed`)) _distancearm))))

(event `Key|MouseScrollUp`
  (params (Key :type "Key Structure" :default "AnyKey"))
  (bind _distancearm (`self.DistanceArm`))
  (bind _targetarmlength (`SpringArmComponent.TargetArmLength` _distancearm))
  (:`Pressed`
    (if (< _targetarmlength 800.0)
      (set `SpringArmComponent.TargetArmLength` (`KismetMathLibrary.FInterpTo` _targetarmlength (+ _targetarmlength (`self.ZoomScale`)) (`GameplayStatics.GetWorldDeltaSeconds`) (`self.ZoomSpeed`)) _distancearm))))

(fn `UserConstructionScript`)